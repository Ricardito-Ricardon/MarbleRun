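; Disco ball enemy character that spots the hero through PawnSensing, flags it on the AI blackboard, and melees with a forward sphere trace, montage and damage.
; Its damage event plays a hit montage, cuts HP and also flags the hero as seen.
; Tick sets blackboard IsDead unconditionally; at zero HP it stops AI and movement, sets the anim death flag, and after a delay destroys itself, adding score and showing a paused win screen at seven.
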(event `self.PawnSensing.OnSeePawn`
  (params (Pawn :type "Pawn Object Reference"))
  ;[1 1 1] Detection
  (cast `/Game/BP_Hero` Pawn)
  (`BlackboardComponent.SetValueAsBool` (`AIBlueprintHelperLibrary.GetBlackboard` (`AIBlueprintHelperLibrary.GetAIController` self)) "hasSeenPlayer?" true))

(event `Attack Player`
  (bind _returnvalue (`self.K2_GetActorLocation`))
  ;[1 1 1] Attack
  (bind _outhit (`KismetSystemLibrary.SphereTraceSingleForObjects` _returnvalue (+ _returnvalue (* (`KismetMathLibrary.GetForwardVector` (`self.K2_GetActorRotation`)) 250.0) (0.0 0.0 0.0)) 120.0 (`|MakeArray` "ObjectTypeQuery3" :!type "EObjectTypeQuery Enum")))
  (if true
    (bind (_bblockinghit _binitialoverlap _time _distance _location _impactpoint _normal _impactnormal _physmat _hitactor) (`GameplayStatics.BreakHitResult` _outhit))
    (cast `/Game/BP_Hero` _hitactor)
    (`self.PlayAnimMontage` "/Game/_MyFiles/Characters/DiscoBall/Animations/SKM_DiscoBall_Attack_Montage.SKM_DiscoBall_Attack_Montage")
    (`GameplayStatics.ApplyDamage` _hitactor 3.0)))

(event `/Game/_MyFiles/Damage/Damage_Interface.ApplyDamage`
  (`|PlayMontage` (`self.Mesh`) "/Game/_MyFiles/Characters/DiscoBall/Animations/SKM_DiscoBall_Damaged_Montage.SKM_DiscoBall_Damaged_Montage"
    (:`then`
      (set `self.HP` (- (`self.HP`) 30))
      (`BlackboardComponent.SetValueAsBool` (`AIBlueprintHelperLibrary.GetBlackboard` (`AIBlueprintHelperLibrary.GetAIController` self)) "hasSeenPlayer?" true))))

(event `self.ReceiveTick`
  (params (DeltaSeconds :type "Float (single-precision)"))
  (bind _returnvalue (`GameplayStatics.GetPlayerController` 0))
  (`|ExecutionSequence`
    (:`then_0`
      (`BlackboardComponent.SetValueAsBool` (`AIBlueprintHelperLibrary.GetBlackboard` (`AIBlueprintHelperLibrary.GetAIController` self)) "IsDead" true)
      (if (<= (`self.HP`) 0)
        (bind _asabp_ai (cast `/Game/_MyFiles/Characters/DiscoBall/Animations/ABP_AI` (`SkeletalMeshComponent.GetAnimInstance` (`self.Mesh`))))
        (set `/Game/_MyFiles/Characters/DiscoBall/Animations/ABP_AI.IsDead` true _asabp_ai)))
    (:`then_1`
      (if (<= (`self.HP`) 0)
        (`CharacterMovementComponent.DisableMovement` (`self.CharacterMovement`))
        (`BrainComponent.StopLogic` (`AIController.BrainComponent` (`AIBlueprintHelperLibrary.GetAIController` self)) "")
        (`KismetSystemLibrary.Delay` 5.0)
        (`self.K2_DestroyActor`)
        (bind _asbp_hero (cast `/Game/BP_Hero` (`GameplayStatics.GetPlayerCharacter` 0)))
        (bind _output_get (set `/Game/BP_Hero.score` (+ (`/Game/BP_Hero.score` _asbp_hero) 1) _asbp_hero))
        (if (== _output_get 7)
          (bind _returnvalue_2 (`|GenericCreateObject` "/Game/_MyFiles/UI/WinUI.WinUI_C"))
          (`UserWidget.AddToViewport` _returnvalue_2 0)
          (`WidgetBlueprintLibrary.SetInputMode_UIOnlyEx` _returnvalue null)
          (set `PlayerController.bShowMouseCursor` true _returnvalue)
          (`GameplayStatics.SetGamePaused` true))))))

(event `self.ReceiveBeginPlay`
  (`BlackboardComponent.SetValueAsBool` (`AIBlueprintHelperLibrary.GetBlackboard` (`AIBlueprintHelperLibrary.GetAIController` self)) "hasSeenPlayer?" false))

(fn `UserConstructionScript`)